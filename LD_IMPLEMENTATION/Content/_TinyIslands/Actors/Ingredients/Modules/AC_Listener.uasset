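; AC_Listener is an actor component that lets its owner switch on or off in response to connected activators.
; It counts required and currently active activators, with inverted activators counting as active when connected and reversing their requests.
; Each request rechecks whether all, or at least one, are active.
; It then calls ActivateListener or DeactivateListener on the owner through BI_Listener, logging if that interface is missing.
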(event Custom|Request%20Deactivation
  (params (isActivatorInverted :type Boolean))
  (bind _returnvalue (Components|GetOwner))
  (if isActivatorInverted
    (Variables|Default|SetActivationCurrentAmount (+ (Variables|Default|GetActivationCurrentAmount) 1))
    (bind _activationstatus (CallFunction|CheckActivationRequirements))
    (Variables|Default|SetIsActivated _activationstatus)
    (else
      (Variables|Default|SetActivationCurrentAmount (- (Variables|Default|GetActivationCurrentAmount) 1))
      (bind _activationstatus_2 (CallFunction|CheckActivationRequirements))
      (Variables|Default|SetIsActivated _activationstatus_2)))
  (if (Utilities|DoesObjectImplementInterface _returnvalue "/Game/_TinyIslands/Actors/Ingredients/Modules/BI_Listener.BI_Listener_C")
    (bind _asbi_listener (Utilities|Casting|CastToBI_Listener _returnvalue))
    (if (Variables|Default|GetIsActivated)
      (Default|ActivateListener _asbi_listener)
      (else
        (Default|DeactivateListener _asbi_listener)))
    (else
      (Utilities|String|LogString "AC_Listener : Parent does not implement BI_Listener interface"))))

(event Custom|Request%20Activation
  (params (isActivatorInverted :type Boolean))
  (bind _returnvalue (Components|GetOwner))
  (if isActivatorInverted
    (Variables|Default|SetActivationCurrentAmount (- (Variables|Default|GetActivationCurrentAmount) 1))
    (bind _activationstatus (CallFunction|CheckActivationRequirements))
    (Variables|Default|SetIsActivated _activationstatus)
    (else
      (Variables|Default|SetActivationCurrentAmount (+ (Variables|Default|GetActivationCurrentAmount) 1))
      (bind _activationstatus_2 (CallFunction|CheckActivationRequirements))
      (Variables|Default|SetIsActivated _activationstatus_2)))
  (if (Utilities|DoesObjectImplementInterface _returnvalue "/Game/_TinyIslands/Actors/Ingredients/Modules/BI_Listener.BI_Listener_C")
    (bind _asbi_listener (Utilities|Casting|CastToBI_Listener _returnvalue))
    (if (Variables|Default|GetIsActivated)
      (Default|ActivateListener _asbi_listener)
      (else
        (Default|DeactivateListener _asbi_listener)))
    (else
      (Utilities|String|LogString "AC_Listener : Parent does not implement BI_Listener interface"))))

(event Custom|Add%20Connected%20Activator
  (params (isActivatorInverted :type Boolean))
  (Variables|Default|SetActivationRequieredAmount (+ (Variables|Default|GetActivationRequieredAmount) 1))
  (if isActivatorInverted
    (Variables|Default|SetActivationCurrentAmount (+ (Variables|Default|GetActivationCurrentAmount) 1))
    (Development|PrintString "Add Inverted")))

(event EventBeginPlay)

(event EventTick
  (params (DeltaSeconds :type Float%20%28single-precision%29)))

(fn CheckActivationRequirements
  (Development|PrintText (Utilities|Text|FormatText "[Req: {required}, Amnt: {amount}]" (Variables|Default|GetActivationRequieredAmount) (Variables|Default|GetActivationCurrentAmount)))
  (if (Variables|Default|GetRequiresAllActivated)
    (LocalVariables|SetActivated (>= (Variables|Default|GetActivationCurrentAmount) (Variables|Default|GetActivationRequieredAmount)))
    (else
      (LocalVariables|SetActivated (>= (Variables|Default|GetActivationCurrentAmount) 1))))
  (return (LocalVariables|GetActivated) false))

(fn UpdateActivationStatus)