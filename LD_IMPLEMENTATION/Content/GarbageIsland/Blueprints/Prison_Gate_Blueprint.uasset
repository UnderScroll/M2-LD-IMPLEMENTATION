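; Prison gate Blueprint that slides its gate component between its starting position and an offset in response to activate and deactivate events.
; BeginPlay caches the relative location of GatePH as the default.
; ActivateListener and DeactivateListener stop the offset timeline, then play or reverse it, so movement can change direction mid-travel.
; Each timeline update adds DoorOffset to that default and sets the location without sweep.
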(event EventBeginPlay
  (Variables|Default|SetDefaultLocation (Variables|/Script/Engine.SceneComponent|GetRelativeLocation (Variables|Default|GetGate_PH))))

(event Collision|EventActorBeginOverlap
  (params (OtherActor :type Actor%20Object%20Reference)))

(event EventTick
  (params (DeltaSeconds :type Float%20%28single-precision%29)))

(event EventActivateListener
  (Audio|Components|Audio|Stop (Variables|Default|GetGate_Offset_Timeline))
  (bind _door_offset (Timeline|Gate_Offset_Timeline Play)
    (:Update
      (Transformation|SetRelativeLocation (Variables|Default|GetGate_PH) (+ (Variables|Default|GetDefaultLocation) _door_offset) false false))))

(event EventDeactivateListener
  (Audio|Components|Audio|Stop (Variables|Default|GetGate_Offset_Timeline))
  (bind _door_offset (Timeline|Gate_Offset_Timeline Reverse)
    (:Update
      (Transformation|SetRelativeLocation (Variables|Default|GetGate_PH) (+ (Variables|Default|GetDefaultLocation) _door_offset) false false))))

(fn ConstructionScript)