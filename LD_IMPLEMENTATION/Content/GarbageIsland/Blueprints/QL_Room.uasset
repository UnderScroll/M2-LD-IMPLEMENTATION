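; QL_Room is a modular room actor for the GarbageIsland game, configured per instance through boolean variables.
; The construction script checks flags for balcony, floor, left wall, right wall, furniture and glass, destroying the matching mesh components when a flag is true.
; Each flag therefore removes its part rather than adding it, and furniture removes a group of three cubes.
; The event graph holds only empty default events, so it adds no runtime logic.
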(event EventBeginPlay)

(event Collision|EventActorBeginOverlap
  (params (OtherActor :type Actor%20Object%20Reference)))

(event EventTick
  (params (DeltaSeconds :type Float%20%28single-precision%29)))

(fn ConstructionScript
  (Utilities|FlowControl|Sequence
    (:then_0
      (if (Variables|Default|GetBalcon)
        (Components|DestroyComponent (Variables|Default|GetCube76_StaticMeshComponent1))))
    (:then_1
      (if (Variables|Default|GetSol)
        (Components|DestroyComponent (Variables|Default|GetCube76_StaticMeshComponent0))))
    (:then_2
      (if (Variables|Default|GetWallLeft)
        (Components|DestroyComponent (Variables|Default|GetCube84_StaticMeshComponent0))))
    (:then_3
      (if (Variables|Default|GetWallRight)
        (Components|DestroyComponent (Variables|Default|GetCube84_StaticMeshComponent1))))
    (:then_4
      (if (Variables|Default|GetFurniture)
        (Components|DestroyComponent (Variables|Default|GetCube))))
    (:then_5
      (if (Variables|Default|GetGlass)
        (Components|DestroyComponent (Variables|Default|GetCube3))))))